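; AIC_Enemy is an AI controller for enemies, currently only a partial setup.
; On BeginPlay it initializes the BB_Enemy blackboard and writes PatrolPoint2 into its patrol point key.
; The nodes to run BT_Enemy, pick a random branch and set a BP_SpaceShip attack target are disconnected, so the controller never starts the behavior tree itself.
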(event EventBeginPlay
  (bind _blackboardcomponent (Class|AIController|UseBlackboard "/Game/Blueprints/AI/BB_Enemy.BB_Enemy"))
  (AI|Components|Blackboard|SetValueasVector _blackboardcomponent (Variables|Default|GetPatrolPointKey) (Variables|Default|GetPatrolPoint_2)))

(event EventTick
  (params (DeltaSeconds :type Float%20%28single-precision%29)))

(fn ConstructionScript)