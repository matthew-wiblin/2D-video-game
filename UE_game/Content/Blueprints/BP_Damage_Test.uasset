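; BP_Damage_Test is a test damage zone that drains health from a BP_SpaceShip inside its sphere.
; On sphere begin overlap, it stores the ship reference and starts a looping timer that calls ReduceHealth every tenth of a second.
; ReduceHealth subtracts a fixed amount straight from the ship's HealthCurrent, with no clamping.
; When a ship leaves the sphere, the timer is cleared by function name.
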(event OnComponentBeginOverlap(Sphere)
  (params (OverlappedComponent :type Primitive%20Component%20Object%20Reference) (OtherActor :type Actor%20Object%20Reference) (OtherComp :type Primitive%20Component%20Object%20Reference) (OtherBodyIndex :type Integer) (bFromSweep :type Boolean) (SweepResult :type Hit%20Result%20Structure%20%28by%20ref%29))
  (bind _asbp_space_ship (Utilities|Casting|CastToBP_SpaceShip OtherActor))
  (Variables|Default|SetPlayerRef _asbp_space_ship)
  (Utilities|Time|SetTimerbyFunctionName 0 "ReduceHealth" 0.1 true))

(event OnComponentEndOverlap(Sphere)
  (params (OverlappedComponent :type Primitive%20Component%20Object%20Reference) (OtherActor :type Actor%20Object%20Reference) (OtherComp :type Primitive%20Component%20Object%20Reference) (OtherBodyIndex :type Integer))
  (Utilities|Casting|CastToBP_SpaceShip OtherActor)
  (Utilities|Time|ClearTimerbyFunctionName 0 "ReduceHealth"))

(event EventBeginPlay)

(event Collision|EventActorBeginOverlap
  (params (OtherActor :type Actor%20Object%20Reference)))

(event EventTick
  (params (DeltaSeconds :type Float%20%28single-precision%29)))

(fn ConstructionScript)

(fn ReduceHealth
  (bind _playerref (Variables|Default|GetPlayerRef))
  (Variables|/Game/Blueprints/Characters/Ship/BP_SpaceShip.BP_SpaceShip_C|SetHealthCurrent _playerref (- (Variables|/Game/Blueprints/Characters/Ship/BP_SpaceShip.BP_SpaceShip_C|GetHealthCurrent _playerref) 4.0)))