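; Red alien enemy that patrols, targets the player's spaceship and drains its health on contact.
; BeginPlay runs BT_Enemy, then keeps writing a random one of four patrol points to the blackboard, polling distance until arrival before picking again.
; Sphere overlaps set or clear the blackboard attack target through AIC_Enemy.
; HitBox overlap starts a looping timer that reduces ship health until the overlap ends.
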(event OnComponentBeginOverlap(HitBox)
  (params (OverlappedComponent :type Primitive%20Component%20Object%20Reference) (OtherActor :type Actor%20Object%20Reference) (OtherComp :type Primitive%20Component%20Object%20Reference) (OtherBodyIndex :type Integer) (bFromSweep :type Boolean) (SweepResult :type Hit%20Result%20Structure%20%28by%20ref%29))
  (bind _asbp_space_ship (Utilities|Casting|CastToBP_SpaceShip OtherActor))
  (Variables|Default|SetPlayerRef _asbp_space_ship)
  (Utilities|Time|SetTimerbyFunctionName 0 "ReduceHealth" 0.1 true))

(event OnComponentEndOverlap(HitBox)
  (params (OverlappedComponent :type Primitive%20Component%20Object%20Reference) (OtherActor :type Actor%20Object%20Reference) (OtherComp :type Primitive%20Component%20Object%20Reference) (OtherBodyIndex :type Integer))
  (Utilities|Casting|CastToBP_SpaceShip OtherActor)
  (Utilities|Time|ClearTimerbyFunctionName 0 "ReduceHealth"))

(event OnComponentBeginOverlap(Sphere)
  (params (OverlappedComponent :type Primitive%20Component%20Object%20Reference) (OtherActor :type Actor%20Object%20Reference) (OtherComp :type Primitive%20Component%20Object%20Reference) (OtherBodyIndex :type Integer) (bFromSweep :type Boolean) (SweepResult :type Hit%20Result%20Structure%20%28by%20ref%29))
  (bind _asbp_space_ship (Utilities|Casting|CastToBP_SpaceShip OtherActor))
  (bind _asaic_enemy (Utilities|Casting|CastToAIC_Enemy (AI|GetAIController self)))
  (bind _blackboardcomponent (Class|AIController|UseBlackboard _asaic_enemy "/Game/Blueprints/AI/BB_Enemy.BB_Enemy"))
  (AI|Components|Blackboard|SetValueasObject _blackboardcomponent (Variables|Default|GetKeyAttackTarget) _asbp_space_ship))

(event OnComponentEndOverlap(Sphere)
  (params (OverlappedComponent :type Primitive%20Component%20Object%20Reference) (OtherActor :type Actor%20Object%20Reference) (OtherComp :type Primitive%20Component%20Object%20Reference) (OtherBodyIndex :type Integer))
  (Utilities|Casting|CastToBP_SpaceShip OtherActor)
  (bind _asaic_enemy (Utilities|Casting|CastToAIC_Enemy (AI|GetAIController self)))
  (bind _blackboardcomponent (Class|AIController|UseBlackboard _asaic_enemy "/Game/Blueprints/AI/BB_Enemy.BB_Enemy"))
  (AI|Components|Blackboard|SetValueasObject _blackboardcomponent (Variables|Default|GetKeyAttackTarget) 0))

(event EventBeginPlay
  (bind _patrolpoint_1 (Variables|Default|GetPatrolPoint_1))
  (bind _patrolpoint_2 (Variables|Default|GetPatrolPoint_2))
  (bind _patrolpoint_3 (Variables|Default|GetPatrolPoint_3))
  (bind _patrolpoint_4 (Variables|Default|GetPatrolPoint_4))
  (|CallParentFunction)
  (bind _asaic_enemy (Utilities|Casting|CastToAIC_Enemy (AI|GetAIController self)))
  (AI|RunBehaviorTree _asaic_enemy "/Game/Blueprints/AI/BT_Enemy.BT_Enemy")
  (bind _blackboardcomponent (Class|AIController|UseBlackboard _asaic_enemy "/Game/Blueprints/AI/BB_Enemy.BB_Enemy"))
  (switch int (Math|Random|RandomInteger 4) :!label _label
    (:0
      (AI|Components|Blackboard|SetValueasVector _blackboardcomponent (Variables|Default|GetPatrolPointKey) _patrolpoint_1)
      (if (> (Math|Vector|Distance(Vector) _patrolpoint_1 (Transformation|GetActorLocation self)) 5e+01) :!label _label_2
        (Utilities|FlowControl|Delay 0.2)
        (goto _label_2)
        (else
          (goto _label))))
    (:1
      (AI|Components|Blackboard|SetValueasVector _blackboardcomponent (Variables|Default|GetPatrolPointKey) _patrolpoint_2)
      (if (> (Math|Vector|Distance(Vector) _patrolpoint_2 (Transformation|GetActorLocation self)) 5e+01) :!label _label_3
        (Utilities|FlowControl|Delay 0.2)
        (goto _label_3)
        (else
          (goto _label))))
    (:2
      (AI|Components|Blackboard|SetValueasVector _blackboardcomponent (Variables|Default|GetPatrolPointKey) _patrolpoint_3)
      (if (> (Math|Vector|Distance(Vector) _patrolpoint_3 (Transformation|GetActorLocation self)) 5e+01) :!label _label_4
        (Utilities|FlowControl|Delay 0.2)
        (goto _label_4)
        (else
          (goto _label))))
    (:3
      (AI|Components|Blackboard|SetValueasVector _blackboardcomponent (Variables|Default|GetPatrolPointKey) _patrolpoint_4)
      (if (> (Math|Vector|Distance(Vector) _patrolpoint_4 (Transformation|GetActorLocation self)) 5e+01) :!label _label_5
        (Utilities|FlowControl|Delay 0.2)
        (goto _label_5)
        (else
          (goto _label))))))

(fn ConstructionScript
  (|CallParentFunction))

(fn ReduceHealth
  (bind _playerref (Variables|Default|GetPlayerRef))
  (Variables|/Game/Blueprints/Characters/Ship/BP_SpaceShip.BP_SpaceShip_C|SetHealthCurrent _playerref (- (Variables|/Game/Blueprints/Characters/Ship/BP_SpaceShip.BP_SpaceShip_C|GetHealthCurrent _playerref) 2.0)))