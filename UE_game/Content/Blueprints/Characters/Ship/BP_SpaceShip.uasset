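; Player-controlled spaceship that moves on the XY plane through Enhanced Input, scores points for survival time and ends the run when health runs out.
; Move input is scaled down on diagonals, and a held boost input doubles the speed multiplier.
; A looping timer adds to the GI_Action score and regenerates health up to max, or flags the game as played and opens the main menu at zero health.
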(event Custom|HighScoreAndEndGame
  (CallFunction|CheckHealthandScoreandEndGame))

(event Input|EnhancedActionEvents|EnhancedInputActionIA_Move
  (params (ActionValue :type Vector%202D%20Structure) (ElapsedSeconds :type Float%20%28double-precision%29) (TriggeredSeconds :type Float%20%28double-precision%29) (InputAction :type Input%20Action%20Object%20Reference :default "/Game/Input/Actions/IA_Move.IA_Move"))
  (bind (_x _y) (Math|Vector2D|BreakVector2D ActionValue))
  (if (and (!= _x 0.0) (!= _y 0.0))
    (Variables|Default|SetSpeed 0.353553)
    (else
      (Variables|Default|SetSpeed 0.5)))
  (Pawn|Input|AddMovementInput (Math|Vector|MakeVector (* (Variables|Default|GetSpeed) (Variables|Default|GetSpeedMultiplier)) 0.0 0.0) _x false)
  (Pawn|Input|AddMovementInput (Math|Vector|MakeVector 0.0 (* (* (Variables|Default|GetSpeed) (Variables|Default|GetSpeedMultiplier)) -1.0) 0.0) _y false))

(event Input|EnhancedActionEvents|EnhancedInputActionIA_SpeedBoost
  (params (ActionValue :type Boolean) (ElapsedSeconds :type Float%20%28double-precision%29) (TriggeredSeconds :type Float%20%28double-precision%29) (InputAction :type Input%20Action%20Object%20Reference :default "/Game/Input/Actions/IA_SpeedBoost.IA_SpeedBoost"))
  (:Started
    (Variables|Default|SetSpeedMultiplier (* (Variables|Default|GetSpeedMultiplier) 2.0)))
  (:Completed
    (Variables|Default|SetSpeedMultiplier (/ (Variables|Default|GetSpeedMultiplier) 2.0))))

(event EventBeginPlay
  (|CallParentFunction)
  (bind _asplayer_controller (Utilities|Casting|CastToPlayerController (Pawn|GetController)))
  (Input|AddMappingContext (PlayerController|LocalPlayerSubsystems|GetEnhancedInputLocalPlayerSubsystem _asplayer_controller) "/Game/Input/IMC_Action.IMC_Action" 0 "(bIgnoreAllPressedKeysUntilRelease=True,bForceImmediately=False,bNotifyUserSettings=False)")
  (Variables|Default|SetHealthCurrent (Variables|Default|GetHealthMax))
  (Utilities|Time|SetTimerbyEvent (delegate Custom|HighScoreAndEndGame) 0.1 true))

(event Collision|EventActorBeginOverlap
  (params (OtherActor :type Actor%20Object%20Reference)))

(event EventTick
  (params (DeltaSeconds :type Float%20%28single-precision%29))
  (|CallParentFunction 0.0))

(fn ConstructionScript
  (|CallParentFunction))

(fn CheckHealthandScoreandEndGame
  (Math|Float|CompareFloat (Variables|Default|GetHealthCurrent) 0.0
    (:>
      (bind _asgi_action (Utilities|Casting|CastToGI_Action (Game|GetGameInstance)))
      (Variables|/Game/Blueprints/GI_Action.GI_Action_C|SetRecentScore _asgi_action (+ (Variables|/Game/Blueprints/GI_Action.GI_Action_C|GetRecentScore _asgi_action) 0.1))
      (Math|Float|CompareFloat (Variables|Default|GetHealthCurrent) (Variables|Default|GetHealthMax)
        (:<
          (if (> (+ (Variables|Default|GetHealthCurrent) 0.5) (Variables|Default|GetHealthMax))
            (Variables|Default|SetHealthCurrent (Variables|Default|GetHealthMax))
            (else
              (Variables|Default|SetHealthCurrent (+ (Variables|Default|GetHealthCurrent) 0.5)))))))
    (:==
      (bind _asgi_action_2 (Utilities|Casting|CastToGI_Action (Game|GetGameInstance) :!label _label))
      (Variables|/Game/Blueprints/GI_Action.GI_Action_C|SetWasGameJustPlayed _asgi_action_2 true)
      (Game|OpenLevel(byName) "MAP_MainMenu"))
    (:<
      (goto _label))))